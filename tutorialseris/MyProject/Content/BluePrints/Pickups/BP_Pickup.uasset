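; BP_Pickup is a side-scroller pickup that spins and bobs, then disappears when the player character touches it.
; On BeginPlay it randomizes the mesh's starting yaw and oscillation frequency so instances move out of sync.
; Tick applies the yaw rotation and a game-time sine-wave vertical offset to the mesh.
; Box overlap with SideScrollerCharacter destroys the actor, with no reward logic in this Blueprint.
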(event OnComponentBeginOverlap(Box)
  (params (OverlappedComponent :type Primitive%20Component%20Object%20Reference) (OtherActor :type Actor%20Object%20Reference) (OtherComp :type Primitive%20Component%20Object%20Reference) (OtherBodyIndex :type Integer) (bFromSweep :type Boolean) (SweepResult :type Hit%20Result%20Structure%20%28by%20ref%29))
  (Utilities|Casting|CastToSideScrollerCharacter OtherActor)
  (Actor|DestroyActor))

(event EventTick
  (params (DeltaSeconds :type Float%20%28single-precision%29))
  (bind _mesh (Variables|Default|GetMesh))
  (Transformation|AddLocalRotation _mesh (Math|Rotator|MakeRotator 0.0 0.0 (Variables|Default|GetPickupRotation)) false false)
  (Transformation|AddLocalOffset _mesh (Math|Vector|MakeVector 0.0 0.0 (* (Math|Trig|Sin(Radians) (* (Utilities|Time|GetGameTimeinSeconds) (Variables|Default|GetOffsetOscillation))) (Variables|Default|GetOffsetMultiplier))) false true))

(event EventBeginPlay
  (Transformation|AddLocalRotation (Variables|Default|GetMesh) (Math|Rotator|MakeRotator 0.0 0.0 (Math|Random|RandomFloatinRange 0.0 359.0)) false false)
  (Variables|Default|SetOffsetOscillation (Math|Random|RandomFloatinRange 5.0 1e+01)))

(fn ConstructionScript)